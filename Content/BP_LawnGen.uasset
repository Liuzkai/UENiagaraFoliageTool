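; BP_LawnGen is a lawn generator actor that pairs an orthographic scene capture with a Niagara spawn system.
; Construction fits the box, decal, capture, helper meshes and Niagara size to OrthoWidth and CaptureHeight, and passes itself to Niagara.
; CaptureNow captures the scene between toggles of an MPC capture flag, after setting a random MPC color.
; ReceiveData unpauses Niagara, while ParticleData only prints the received particle count.
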(event `CaptureNow`
  (bind _scenecapturecomponent2d (`self.SceneCaptureComponent2D`))
  (`KismetMaterialLibrary.SetScalarParameterValue` "/UENiagaraFoliageTool/Data/MPC_LawnGen.MPC_LawnGen" "capture" 1.0)
  (set `self.Linear Color` (make `LinearColor` (`KismetMathLibrary.RandomFloatInRange` 0.0 1.0) (`KismetMathLibrary.RandomFloatInRange` 0.0 1.0) (`KismetMathLibrary.RandomFloatInRange` 0.0 1.0) 1.0))
  (`KismetMaterialLibrary.SetVectorParameterValue` "/UENiagaraFoliageTool/Data/MPC_LawnGen.MPC_LawnGen" "Color" (`self.Linear Color`))
  (set `SceneCaptureComponent2D.OrthoWidth` (`self.Ortho Width`) _scenecapturecomponent2d)
  (`SceneCaptureComponent2D.CaptureScene` _scenecapturecomponent2d)
  (`KismetMaterialLibrary.SetScalarParameterValue` "/UENiagaraFoliageTool/Data/MPC_LawnGen.MPC_LawnGen" "capture"))

(event `self.ReceiveParticleData`
  (params (Data :type "Array of BasicParticleData Structure (by ref)") (NiagaraSystem :type "NiagaraSystem Object Reference"))
  (`KismetSystemLibrary.PrintString` (`KismetStringLibrary.Conv_IntToString` (`KismetArrayLibrary.Array_Length` Data))))

(event `ReceiveData`
  (`NiagaraComponent.SetPaused` (`self.NS_Spawn`) false))

(fn `UserConstructionScript`
  (bind _ortho_width (`self.Ortho Width`))
  (bind _capture_height (`self.Capture Height`))
  (bind _returnvalue (/ (`self.Ortho Width`) 2.0))
  (bind _returnvalue_2 (- _returnvalue 50.0))
  (bind _returnvalue_3 (- _returnvalue 50.0))
  (`|ExecutionSequence`
    (:`then_0`
      (`NiagaraComponent.SetVariableObject` (`self.NS_Spawn`) "Object" self))
    (:`then_1`
      (`BoxComponent.SetBoxExtent` (`self.Box`) (`KismetMathLibrary.MakeVector` _returnvalue _returnvalue 100.0) true)
      (`SceneComponent.SetWorldScale3D` (`self.Decal`) (`KismetMathLibrary.MakeVector` 1.0 _returnvalue _returnvalue))
      (`SceneComponent.K2_SetRelativeLocation` (`self.SceneCaptureComponent2D`) (`KismetMathLibrary.MakeVector` 0.0 0.0 (`self.Capture Height`)) false false)
      (`SceneComponent.K2_SetRelativeLocation` (`self.StaticMesh`) (`KismetMathLibrary.MakeVector` _returnvalue_2 _returnvalue_3 (+ _capture_height 1.0)) false false)
      (`SceneComponent.K2_SetRelativeLocation` (`self.CapturePaint`) (`KismetMathLibrary.MakeVector` _returnvalue_2 _returnvalue_3 (+ _capture_height 1000.0)) false false)
      (`NiagaraComponent.SetVariableVec3` (`self.NS_Spawn`) "GobalSize" (`KismetMathLibrary.MakeVector` _ortho_width _ortho_width 1.0)))))